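; AgroCheck is a behavior tree node for passerby AI, meant to spot nearby targets to follow.
; Each tick it caches the BP_AICON controller and sphere-traces around its pawn, ignoring all AI_Passerby actors.
; The hit loop is empty: the line-of-sight trace that would set or update the TargetToFollow and TargetLocation blackboard keys is disconnected, so no target is ever written.
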(event EventTick
  (params (OwnerActor :type Actor%20Object%20Reference) (DeltaSeconds :type Float%20%28single-precision%29))
  ;[1 1 1] Is BP_AICON set?
  (if (!= (Variables|Default|GetAI_CON_Ref) 0)
    _
    (else
      (bind _asbp_aicon (Utilities|Casting|CastToBP_AICON OwnerActor))
      (Variables|Default|SetAI_CON_Ref _asbp_aicon)))
  (bind _outactors (Actor|GetAllActorsOfClass "/Game/BluePrints/Passerby_AI/AI_Passerby.AI_Passerby_C"))
  (Variables|Default|SetMyLocation (Transformation|GetActorLocation (Pawn|GetControlledPawn (Variables|Default|GetAI_CON_Ref))))
  (bind _outhits (Collision|MultiSphereTraceForObjects (Transformation|GetActorLocation (Pawn|GetControlledPawn (Variables|Default|GetAI_CON_Ref))) (+ (Transformation|GetActorLocation (Pawn|GetControlledPawn (Variables|Default|GetAI_CON_Ref))) "0, 0,15.000000") 1.5e+03 "ObjectTypeQuery1" false _outactors "None"))
  (bind _array_element (Utilities|Array|ForEachLoopwithBreak _outhits)))