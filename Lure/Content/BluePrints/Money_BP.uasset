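; Money_BP is an actor that places itself near the player on spawn and can be moved and turned by keyboard.
; BeginPlay scales it up, enables input and offsets it from the player, adding 100 to the flattened forward vector rather than multiplying.
; Tick caches its location, which Z and X presses shift along its forward axis using Tick's delta time.
; J adds a fixed yaw step; a separate RotationScale update never runs.
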(event Collision|EventActorBeginOverlap
  (params (OtherActor :type Actor%20Object%20Reference)))

(event EventBeginPlay
  (bind _returnvalue (Game|GetPlayerCharacter 0))
  (bind _returnvalue_2 (Transformation|GetActorLocation _returnvalue))
  (bind _rootcomponent (Variables|/Script/Engine.Actor|GetRootComponent _returnvalue))
  (bind _returnvalue_3 (Math|Vector|GetForwardVector _rootcomponent))
  ;[1 1 1] Player start location, set to a fixed distance from player
  (Development|PrintString "Spawned shit")
  (Transformation|SetActorScale3D "8.000000,8.000000,20.000000")
  (Input|EnableInput (Game|GetPlayerController 0))
  (bind _output_get (Variables|Default|SetCurrent%20Location (+ (Math|Vector|MakeVector (.x _returnvalue_2) (.y _returnvalue_2) 3e+01) (+ (Math|Vector|MakeVector (.x _returnvalue_3) (.y _returnvalue_3) 0.0) 1e+02))))
  (Transformation|SetActorLocation _output_get false false)
  (Variables|Default|SetrotationScale 0.0))

(event EventTick
  (params (DeltaSeconds :type Float%20%28single-precision%29))
  ;[1 1 1] Key presses, update the current location every frame and add offset to current location according to key presses
  (Variables|Default|SetcurrentRotation (Math|Rotator|GetRotationXVector (Transformation|GetActorRotation)))
  (Variables|Default|SetCurrent%20Location (Transformation|GetActorLocation)))

(event Input|KeyboardEvents|Z
  (params (Key :type Key%20Structure))
  ;[1 1 1] Key presses, update the current location every frame and add offset to current location according to key presses
  (:Pressed
    (Transformation|SetActorLocation (+ (* (Transformation|GetActorForwardVector) (* (stale EventTick DeltaSeconds) 5e+03)) (Variables|Default|GetCurrent%20Location)) false false)))

(event Input|KeyboardEvents|J
  (params (Key :type Key%20Structure))
  (bind _returnvalue (Transformation|GetActorRotation))
  (:Pressed
    (Transformation|SetActorRotation (Math|Rotator|MakeRotator (.roll _returnvalue) (.pitch _returnvalue) (+ (.yaw _returnvalue) 3e+01)))))

(event Input|KeyboardEvents|X
  (params (Key :type Key%20Structure))
  ;[1 1 1] Key presses, update the current location every frame and add offset to current location according to key presses
  (:Pressed
    (Transformation|SetActorLocation (+ (Variables|Default|GetCurrent%20Location) (* (Transformation|GetActorForwardVector) (* -5e+03 (stale EventTick DeltaSeconds)))) false false)))

(fn ConstructionScript)