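; BP_WalkingAI is an AI pawn meant to walk a looping route between BP_AIPatrolPoints actors.
; On BeginPlay it gathers those actors and calls GetNextLocation, which increments the patrol index and wraps it to zero past the end.
; A Timeline-driven AI MoveTo would advance the index on arrival, with a two-second re-trigger guard.
; That movement chain is never triggered, so the graph as written does not move the pawn.
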(event EventBeginPlay
  ;[1 1 1] GetPatrolPoints
  (bind _outactors (Actor|GetAllActorsOfClass "/Game/BluePrints/BP_AIPatrolPoints.BP_AIPatrolPoints_C"))
  (Variables|Default|SetPatrolPoints _outactors)
  (CallFunction|GetNextLocation))

(fn ConstructionScript)

(fn GetNextLocation
  (bind _output_get (Variables|Default|SetCurrentPatrolPoints (+ (Variables|Default|GetCurrentPatrolPoints) 1)))
  (Math|Integer|CompareInt _output_get (Utilities|Array|Length (Variables|Default|GetPatrolPoints))
    (:>
      _)
    (:==
      _))
  (Variables|Default|SetCurrentPatrolPoints 0))