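; Behavior tree node that supplies the next destination for a patrolling AI.
; Each tick it gathers all BP_AIPatrolPoints actors, writes their count to IOverallPoint, and copies the location of the one indexed by ICurrentPoint into VTargetLocation.
; It only reads the current index, and patrol order follows the unsorted GetAllActorsOfClass result.
; The owner is cast to AI_Patrol_CON and cached on first use.
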(event EventTick
  (params (OwnerActor :type Actor%20Object%20Reference) (DeltaSeconds :type Float%20%28single-precision%29))
  (if (!= (Variables|Default|GetAI_CON) 0)
    _
    (else
      (bind _asai_patrol_con (Utilities|Casting|CastToAI_Patrol_CON OwnerActor))
      (Variables|Default|SetAI_CON _asai_patrol_con)))
  (bind _outactors (Actor|GetAllActorsOfClass "/Game/BluePrints/BP_AIPatrolPoints.BP_AIPatrolPoints_C"))
  (Class|BTFunctionLibrary|SetBlackboardValueasInt (Variables|Default|Geti_OverallPoint) (Utilities|Array|Length _outactors))
  (AI|BehaviorTree|SetBlackboardValueasVector (Variables|Default|Getv_TargetLocation) (Transformation|GetActorLocation (Utilities|Array|Get(acopy) _outactors (Class|BTFunctionLibrary|GetBlackboardValueasInt (Variables|Default|Geti_CurrentPoint))))))