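; AI character that patrols TargetPoints, roams or chases the player, chosen by a state enum at BeginPlay.
; Pawn sensing sends it to Food, which paralyzes it, or to Money, which stops alert buildup.
; Seeing the player raises a Tick-driven alert, shown by a reddening sprite, until it flees to a fixed location; alert decays out of sight.
; Events also handle snapping into traps and shrink-or-grow timeline scaling before destruction when eaten.
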(event OnSeePawn(PawnSensing)
  (params (Pawn :type Pawn%20Object%20Reference))
  ;[1 1 1] Find Food
  (Utilities|FlowControl|Sequence
    (:then_0
      (if (Actor|ActorHasTag Pawn "Food") ; If it is food
        (if (== (Variables|Default|GetSeenObject) 0) ; If it already seen something
          (Variables|Default|SetSeenObject Pawn)
          (AI|AIMoveTo self "0, 0, 0" Pawn 5.0 true
            (:OnSuccess
              (CallFunction|Paralyze)
              (bind _asposion_food (Utilities|Casting|CastToPosionFood Pawn)
                (:then
                  (Default|FinishFood _asposion_food))
                (:CastFailed
                  (Development|PrintString "Warn: this is not poison food"))))))))
    (:then_1
      ;[1 1 1] Walk to Money
      (if (Actor|ActorHasTag Pawn "Money")
        (Variables|Default|Setb_SeeMoney true)
        (AI|AIMoveTo self "0, 0, 0" Pawn 5.0 true)))
    (:then_2
      ;[1 1 1] If see player
      (if (Actor|ActorHasTag Pawn "Player")
        (Utilities|FlowControl|Sequence
          (:then_0
            (Variables|Default|Setb_seePlayer true))
          (:then_1
            (Utilities|FlowControl|RetriggerableDelay 0.6)
            (Variables|Default|Setb_seePlayer false)))))))

(event Custom|Roam
  (bind _returnvalue (Transformation|GetActorLocation))
  (bind _self self)
  (bind _randomlocation (Class|NavigationSystemV1|GetRandomPointinNavigableRadius _returnvalue 5e+02 0 0))
  ;[1 1 1] Roam
  (bind (_outhit _returnvalue_2) (Collision|LineTraceByChannel (Transformation|GetActorLocation) _randomlocation "TraceTypeQuery1" false 0 "None"))
  (if _returnvalue_2
    (AI|AIMoveTo _self (.Location (Collision|BreakHitResult _outhit)) 0 5.0 false
      (:OnSuccess
        _)
      (:OnFail
        _))
    (else
      (AI|AIMoveTo _self _randomlocation 0 5.0 false
        (:OnSuccess
          _)
        (:OnFail
          _))))
  (if (not (Variables|Default|Getb_Paralyze))
    (Utilities|FlowControl|Delay 2.0)
    (CallFunction|Roam)))

(event Custom|Chase
  ;[1 1 1] Chase
  (AI|AIMoveTo self "0, 0,0.000000" (Game|GetPlayerCharacter 0) 5.0 false
    (:OnSuccess
      (if (not (Variables|Default|Getb_Paralyze))
        (Utilities|FlowControl|Delay 2.0)
        (CallFunction|Chase)))))

(event Custom|Patrol
  ;[1 1 1] Patrol
  (AI|AIMoveTo self "0, 0, 0" (Utilities|Array|Get(acopy) (Variables|Default|GetTargetPoints) (Variables|Default|Geti_currTarget)) 5.0 false
    (:OnSuccess
      (if (not (Variables|Default|Getb_Paralyze))
        (Utilities|FlowControl|Delay 2.0)
        (CallFunction|NextPoint)
        (CallFunction|Patrol)))))

(event Custom|Paralyze
  ;[1 1 1] Paralyze
  (Components|Movement|StopMovementImmediately (Variables|Character|GetCharacterMovement))
  (Variables|Default|Setb_Paralyze true)
  (Utilities|FlowControl|Delay 4.0)
  (Components|Animation|PlayAnimation (Variables|Character|GetMesh) "/Game/Mannequin/Animations/Death_1.Death_1" false))

(event Custom|RunAwayFromPlayer
  ;[1 1 1] Run away from player
  (Variables|/Script/Engine.CharacterMovementComponent|SetMaxWalkSpeed (Variables|Character|GetCharacterMovement) 6e+02)
  (Components|Animation|PlayAnimation (Variables|Character|GetMesh) "/Game/Mannequin/Animations/ThirdPersonRun.ThirdPersonRun" true)
  (AI|AIMoveTo self (Math|Vector|MakeVector -1.7e+03 -1.2e+03 226.0) 0 5.0 false
    (:OnSuccess
      (Development|PrintString "Success")
      (Components|Animation|SetAnimationMode (Variables|Character|GetMesh) "AnimationBlueprint"))))

(event Custom|GetTrapped
  (params (TrapCenter :type Vector))
  (bind (_x _y) (Math|Vector|BreakVector TrapCenter))
  ;[1 1 1] Get Trap
  (Components|Movement|StopMovementImmediately (Variables|Character|GetCharacterMovement))
  (Transformation|SetActorLocation (Math|Vector|MakeVector _x _y (.Z (Math|Vector|BreakVector (Transformation|GetActorLocation)))) false false)
  (Variables|Default|Setb_Trapped true))

(event Custom|Start
  ;[1 1 1] Set Up
  (bind _outactors (Actor|GetAllActorsOfClass "/Script/Engine.TargetPoint"))
  (Variables|Default|SetTargetPoints _outactors)
  (Variables|Default|Seti_TotalPoint (Utilities|Array|Length _outactors))
  (CallFunction|StartMoving))

(event Custom|BeingEat
  ;[1 1 1] Begin being eat
  (bind _newtrack_1 (Timeline|Eat PlayFromStart)
    (:Update
      (Transformation|SetWorldScale3D (Variables|Collision|GetCapsuleComponent) _newtrack_1))
    (:Finished
      (Actor|DestroyActor))))

(event EventBeginPlay
  ;[1 1 1] Set Up
  (CallFunction|Start))

(event EventTick
  (params (DeltaSeconds :type Float%20%28single-precision%29))
  (bind _returnvalue (Utilities|Time|GetWorldDeltaSeconds))
  (bind _asmy_game_mode (Utilities|Casting|CastTomy_GameMode (Game|GetGameMode)))
  ;[1 1 1] Tick and parameters
  (if (Variables|Default|Getb_seePlayer)
    ;[1 1 1] In vision increase alert
    (if (not (Variables|Default|Getb_SeeMoney))
      (if true
        (Variables|Default|Setf_AlertValue (+ (Variables|Default|Getf_AlertValue) (* (Variables|/Game/ThirdPersonBP/Blueprints/my_GameMode.my_GameMode_C|Getf_AlertIncreaseValue _asmy_game_mode) _returnvalue)))
        (Sprite|SetSpriteColor (Variables|Default|GetPaperSprite) (Math|Color|MakeColor 1.0 (- 1.0 (/ (Variables|Default|Getf_AlertValue) 1e+02)) (- 1.0 (/ (Variables|Default|Getf_AlertValue) 1e+02))) :!label _label)
        (Utilities|FlowControl|Sequence
          (:then_0
            ;[1 1 1] Alert and run away
            (if (>= (Variables|Default|Getf_AlertValue) 95.0)
              (Rendering|Components|Sprite|SetSprite (Variables|Default|GetPaperSprite) "/Game/Images/ExclamationMark.ExclamationMark")
              (CallFunction|RunAwayfromPlayer)))
          (:then_1
            ;[1 1 1] Set sprite visibility
            (Rendering|SetVisibility (Variables|Default|GetPaperSprite) (>= (Variables|Default|Getf_AlertValue) 5.0) false)))))
    (else
      ;[1 1 1] Not in vison, reduce alert
      (if (> (Variables|Default|Getf_AlertValue) 0.0)
        (Variables|Default|Setf_AlertValue (- (Variables|Default|Getf_AlertValue) (* _returnvalue 1e+01)))
        (goto _label)))))

(fn ConstructionScript)

(fn NextPoint
  (bind _result (Math|Integer|IncrementInt (Variables|Default|Geti_currTarget))
    (:%20%20
      (Variables|Default|Seti_currTarget (Math|Integer|%(Integer) _result (Variables|Default|Geti_TotalPoint))))))

(fn StartMoving
  (switch Utilities|FlowControl|Switch|SwitchonEAIState (Variables|Default|GetAIStae)
    (:NewEnumerator1
      (CallFunction|Roam))
    (:NewEnumerator2
      (CallFunction|Chase))
    (:NewEnumerator3
      (CallFunction|Patrol))))