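; Money Lure pawn that can be moved by movement input and visually tethered by a rope beam.
; Forward and backward events apply half-scaled input along a supplied vector, while a separate Move function applies it unscaled.
; The Money component gets gravity enabled on BeginPlay.
; SetBeam spawns a beam particle at RopeAttach, stores it and sets its end point to the given target location.
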(event Custom|SetBeam
  (params (TargetLocation :type Vector))
  ;[1 1 1] Set Rope Spawn and end points
  (bind _returnvalue (Effects|SpawnEmitterAttached "/Game/ParticleSystem/Beam_Particle.Beam_Particle" (Variables|Default|GetRopeAttach) "" "0, 0, 0" "0, 0, 0" "0.100000,0.100000,0.200000"))
  (bind _output_get (Variables|Default|SetRopeAttached _returnvalue))
  (Class|ParticleSystemComponent|SetBeamEndPoint _output_get 0 TargetLocation))

(event Custom|MovePawnForward
  (params (AxisValue :type Float%20%28single-precision%29) (Forward%20Vector :type Vector))
  ;[1 1 1] Pawn Movement
  (Pawn|Input|AddMovementInput Forward%20Vector (* AxisValue 0.5) false))

(event Custom|Move%20Pawn%20Backward
  (params (Axis%20value :type Float%20%28single-precision%29) (Forward%20vector :type Vector))
  ;[1 1 1] Pawn Movement
  (Pawn|Input|AddMovementInput Forward%20vector (* Axis%20value 0.5) false))

(event EventBeginPlay
  (Physics|SetEnableGravity (Variables|Default|GetMoney) true))

(fn ConstructionScript)

(fn Move
  (params (Axis%20value :type Float%20%28single-precision%29) (Direction :type Vector))
  (Pawn|Input|AddMovementInput Direction Axis%20value false))